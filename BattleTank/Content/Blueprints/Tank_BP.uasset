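; Tank Blueprint that sets up the barrel and turret references and handles player camera aiming.
; On BeginPlay it passes its TankBarrel and TankTurret to SetBarrelReference and SetTurretReference.
; The AimAzimuth axis yaws an AzimuthGimbal and AimElevation pitches the SpringArm, keeping the two rotations on separate components.
; Aim input is applied per axis event without delta-time scaling, and this graph does not rotate the barrel or turret.
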(event EventBeginPlay
  (Class|Tank|SetBarrelReference (Variables|Default|GetTank%20Barrel))
  (Class|Tank|SetTurretReference (Variables|Default|GetTank%20Turret)))

(event Input|AxisEvents|InputAxisAimAzimuth
  (params (AxisValue :type Float%20%28single-precision%29))
  ;[1 1 1] Rotation on X Axis
  (Transformation|AddLocalRotation (Variables|Default|GetAzimuth%20Gimbal) (Math|Rotator|MakeRotator 0.0 0.0 (* AxisValue 1.0)) false false))

(event Input|AxisEvents|InputAxisAimElevation
  (params (AxisValue :type Float%20%28single-precision%29))
  ;[1 1 1] Rotation on Y Axis
  (Transformation|AddLocalRotation (Variables|Default|GetSpringArm) (Math|Rotator|MakeRotator 0.0 (* AxisValue 1.0) 0.0) false false))

(fn ConstructionScript)